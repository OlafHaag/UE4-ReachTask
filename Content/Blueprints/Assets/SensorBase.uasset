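; SensorBase is a sensor Blueprint, apparently meant as a base, with a selectable Box or Sphere shape.
; The construction script switches on Shape to show the matching shape and collision components and set that collision to query and physics.
; It only enables the chosen pair and never hides or disables the other, so it relies on component defaults.
; The event graph holds only empty placeholder events, so no detection logic lives here.
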(event EventBeginPlay)

(event Collision|EventActorBeginOverlap
  (params (OtherActor :type Actor%20Object%20Reference)))

(event EventTick
  (params (DeltaSeconds :type Float%20%28single-precision%29)))

(fn ConstructionScript
  (bind _boxcollision (Variables|Default|GetBoxCollision))
  (bind _spherecollision (Variables|Default|GetSphereCollision))
  (switch Utilities|FlowControl|Switch|SwitchonSensorShapesEnum (Variables|Setup|GetShape)
    (:NewEnumerator0
      (Rendering|SetVisibility (Variables|Default|GetBox) true false)
      (Collision|SetCollisionEnabled _boxcollision "QueryAndPhysics")
      (Rendering|SetVisibility _boxcollision true false))
    (:NewEnumerator1
      (Rendering|SetVisibility (Variables|Default|GetSphere) true false)
      (Collision|SetCollisionEnabled _spherecollision "QueryAndPhysics")
      (Rendering|SetVisibility _spherecollision true false))))