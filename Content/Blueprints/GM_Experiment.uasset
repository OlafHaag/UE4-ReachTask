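; Game mode for a trial-based experiment that sets up the session and starts the trials.
; In debug it possesses a spawned debug pawn and views through a spawned camera.
; It loads participant info from a save slot, calls an activator by handedness, then fires trial begin, continuing even without a save.
; A looping timer is meant to record tracker movement until EndPlay, but currently only prints a debug message once.
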(event Custom|Trial%20Begin_Event
  (Development|PrintString "Trial Begin"))

(event Custom|Save%20Movement%20Data
  ;[1 1 1] Movement Recording
  ;;[0.5507 1 0.5938] Debug. ToDo: Record Tracker Movement
  (Utilities|FlowControl|DoOnce false
    (:Completed
      (Development|PrintString "DEBUG: Movement Recording started." true true "(R=1.000000,G=0.000000,B=0.690145,A=1.000000)"))))

(event Custom|ReadyToStart
  ;[1 1 1] ready to start trials
  (bind _returnvalue (Utilities|Time|SetTimerbyEvent (delegate Custom|Save%20Movement%20Data) (Variables|GameSettings|GetMovementRecDeltaTime) true))
  (Variables|Movement|SetMovementRecTimer _returnvalue)
  (CallFunction|TrialBeginEvent :!pinned true) ; Begin trial
)

(event EventBeginPlay
  (bind _returnvalue (Game|GetPlayerController 0))
  ;[1 0.2059 0.0075] Debug Version?
  (bind _asgame_info_instance (Utilities|Casting|CastToGameInfoInstance (Game|GetGameInstance)))
  (bind _output_get (Variables|Game|SetIsDebug? (or (Variables|/Game/Blueprints/GameInfoInstance.GameInfoInstance_C|GetIsDebug? _asgame_info_instance) (Variables|Game|GetIsDebug?))))
  (if _output_get
    (Development|PrintString "DEBUG Version!" true true "(R=1.000000,G=0.000000,B=0.000000,A=1.000000)" 6.0)
    (bind _returnvalue_2 (Game|SpawnActorfromClass "/Game/Blueprints/DebugPawn.DebugPawn_C" (Math|Transform|MakeTransform "-100.000000, 0,50.000000") "Undefined" 0 0))
    (Pawn|Possess _returnvalue _returnvalue_2)
    (bind _returnvalue_3 (Game|SpawnActorfromClass "/Script/Engine.CameraActor" (Math|Transform|MakeTransform "0, 0,500.000000" "-90.000000, 0, 0") "Undefined" 0 0))
    (Game|Player|SetViewTargetwithBlend _returnvalue _returnvalue_3 0.0 "VTBlend_Linear" 0.0 false))
  ;[1 1 1] Load Participant Settings
  (bind _returnvalue_4 (SaveGame|DoesSaveGameExist (Variables|PlayerSettings|GetPlayerSettingsSave)))
  (if _returnvalue_4
    (bind _returnvalue_5 (SaveGame|LoadGamefromSlot (Variables|PlayerSettings|GetPlayerSettingsSave)))
    (bind _assave_player_info (Utilities|Casting|CastToSave_PlayerInfo _returnvalue_5))
    (bind _output_get_2 (Variables|PlayerSettings|SetSaveGameRef _assave_player_info))
    (bind _output_get_3 (Variables|PlayerSettings|SetPlayerInfo (Variables|/Game/Blueprints/Save_PlayerInfo.Save_PlayerInfo_C|GetPlayerInfo _output_get_2)))
    ;[1 1 1] Set Activator by handedness
    (Default|CallCallActivator (Utilities|Struct|BreakPlayerInfo _output_get_3))
    (else
      ;[1 0 0] DEBUG
      (Development|PrintString "Error: No saved participant Info!" true true "(R=1.000000,G=0.000000,B=0.000000,A=1.000000)" 4.0)))
  (CallFunction|ReadytoStart))

(event EventEndPlay
  (params (EndPlayReason :type EEndPlayReason%20Enum :default "Destroyed"))
  ;[1 1 1] Movement Recording
  ;;[1 0.2039 0.2219] Stop Movement Recording
  (Utilities|Time|ClearandInvalidateTimerbyHandle (Variables|Movement|GetMovementRecTimer)))

(fn ConstructionScript)