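; GameInfoInstance, by name a game instance, opens menu widgets such as the main menu through a ShowMainMenu event.
; ShowMenuWidget caches each widget in a Menus map keyed by class, creating it on first request and reusing it afterwards.
; It adds the widget to the viewport, then shows the mouse cursor and switches player 0 to UI-only input without mouse lock.
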(event Custom|ShowMainMenu
  ;[1 1 1] Show Main Menu
  (CallFunction|ShowMenuWidget "/Game/Menu/MainMenu.MainMenu_C"))

(fn ShowMenuWidget
  (params (Widget%20Class :type User%20Widget%20Class%20Reference))
  (bind _returnvalue (Game|GetPlayerController 0))
  (bind _menus (Variables|Default|GetMenus))
  (bind (_value _returnvalue_2) (Utilities|Map|Find _menus Widget%20Class))
  (if _returnvalue_2
    (UserInterface|Viewport|AddtoViewport _value 0)
    (else
      (bind _returnvalue_3 (UserInterface|CreateWidget Widget%20Class _returnvalue))
      (Utilities|Map|Add (Variables|Default|GetMenus) Widget%20Class _returnvalue_3)
      (UserInterface|Viewport|AddtoViewport _returnvalue_3 0)))
  (Variables|/Script/Engine.PlayerController|SetbShowMouseCursor _returnvalue true)
  (Input|SetInputModeUIOnly _returnvalue 0 "DoNotLock"))